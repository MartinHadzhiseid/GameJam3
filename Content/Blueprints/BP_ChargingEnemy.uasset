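; Charging enemy character that moves straight at the player (BP_DuffMcKagan) every tick, deals contact damage and dies when its health runs out.
; Tick steers toward the player reference cached at BeginPlay and flips the mesh to face left or right along X.
; DamageBox overlap damages and launches the player, with a delayed flag as attack cooldown.
; ApplyDamage reduces health; at zero it disables collision and destroys the actor after a brief delay.
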(event OnComponentBeginOverlap(DamageBox)
  (params (OverlappedComponent :type Primitive%20Component%20Object%20Reference) (OtherActor :type Actor%20Object%20Reference) (OtherComp :type Primitive%20Component%20Object%20Reference) (OtherBodyIndex :type Integer) (bFromSweep :type Boolean) (SweepResult :type Hit%20Result%20Structure%20%28by%20ref%29))
  ;[0.15 0.15 0.15 0.5] Deal Damage and Knockback
  (bind _asbp_duff_mc_kagan (Utilities|Casting|CastToBP_DuffMcKagan OtherActor))
  (if (== (Variables|Default|GetIsAttacking) false)
    (Variables|Default|SetIsAttacking true)
    (Class|BPIDamage|ApplyDamage(Message) _asbp_duff_mc_kagan 1e+01)
    (Character|LaunchCharacter (Variables|Default|GetPlayerRef) (Math|Vector|MakeVector (* (.X (Math|Vector|BreakVector (Transformation|GetActorForwardVector))) -2e+03) 0.0 0.0) true true)
    (Development|PrintString "Helloooo")
    (Utilities|FlowControl|Delay 1.0)
    (Variables|Default|SetIsAttacking false)))

(event EventBeginPlay
  ;[0.15 0.15 0.15 0.5] Gets the Player
  (Variables|Default|SetCurrentHealth (Variables|Default|GetMaxHealth))
  (bind _asbp_duff_mc_kagan (Utilities|Casting|CastToBP_DuffMcKagan (Game|GetPlayerCharacter 0)))
  (Variables|Default|SetPlayerRef _asbp_duff_mc_kagan))

(event EventApplyDamage
  (params (DamageAmount :type Float%20%28double-precision%29))
  ;[0.15 0.15 0.15 0.5] Taking Damage and Handling Death
  (bind _output_get (Variables|Default|SetCurrentHealth (Math|Float|Clamp(Float) (- (Variables|Default|GetCurrentHealth) DamageAmount) 0.0 (Variables|Default|GetMaxHealth))))
  (if (<= _output_get 0.0)
    (Components|Movement|StopMovementImmediately (Variables|Character|GetCharacterMovement))
    (Collision|SetCollisionEnabled (Variables|Collision|GetCapsuleComponent) "NoCollision")
    (Collision|SetCollisionEnabled (Variables|Default|GetDamageBox) "NoCollision")
    (Animation|PlayAnimMontage 0 1.0 "None")
    (Utilities|FlowControl|Delay 0.2)
    (Actor|DestroyActor)))

(event EventTick
  (params (DeltaSeconds :type Float%20%28single-precision%29))
  (bind _mesh (Variables|Character|GetMesh))
  ;[0.15 0.15 0.15 0.5] Moves Towards the Player
  (Pawn|Input|AddMovementInput (* (Math|Vector|Normalize (- (Transformation|GetActorLocation (Variables|Default|GetPlayerRef)) (Transformation|GetActorLocation))) (Variables|Default|GetMoveSpeed)) 1.0 false)
  (if (< (.X (Math|Vector|BreakVector (Transformation|GetActorLocation (Variables|Default|GetPlayerRef)))) (.X (Math|Vector|BreakVector (Transformation|GetActorLocation))))
    (Transformation|SetRelativeRotation _mesh "0.000000,90.000000,0.000000" false false)
    (else
      (Transformation|SetRelativeRotation _mesh "0.000000,-90.000000,0.000000" false false))))

(fn ConstructionScript)