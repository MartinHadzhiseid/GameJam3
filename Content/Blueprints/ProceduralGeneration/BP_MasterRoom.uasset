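; BP_MasterRoom is the starting room that procedurally builds a linear chain of rooms when play begins.
; GenerateRooms spawns RoomsToGenerate random picks from the Rooms array, placing each at the previous room's Exit component transform and printing its name.
; ExitPos carries that transform along the chain, so BP_Exit_Room then spawns at the final exit to cap the layout, with no overlap checks in the graph.
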(event EventBeginPlay
  (Variables|Default|SetExitPos (Transformation|GetWorldTransform (Variables|Default|GetExit)))
  (Utilities|FlowControl|Sequence
    (:then_0
      (CallFunction|GenerateRooms))
    (:then_1
      (Game|SpawnActorfromClass "/Game/Blueprints/ProceduralGeneration/BP_Exit_Room.BP_Exit_Room_C" (Variables|Default|GetExitPos) "Undefined" "MultiplyWithRoot" 0 0))))

(event Collision|EventActorBeginOverlap
  (params (OtherActor :type Actor%20Object%20Reference)))

(event EventTick
  (params (DeltaSeconds :type Float%20%28single-precision%29)))

(fn ConstructionScript)

(fn GenerateRooms
  (for _index (range 1 (Variables|Default|GetRoomsToGenerate))
    (bind _returnvalue (Game|SpawnActorfromClass (Utilities|Array|Get(acopy) (Variables|Default|GetRooms) (Math|Random|RandomInteger (Utilities|Array|Length (Variables|Default|GetRooms)))) (Variables|Default|GetExitPos) "Undefined" "MultiplyWithRoot" 0 0))
    (Development|PrintString (Utilities|String|ToString(Object) _returnvalue))
    (Variables|Default|SetExitPos (Transformation|GetWorldTransform (Variables|/Game/Blueprints/ProceduralGeneration/BP_Base_Room.BP_Base_Room_C|GetExit _returnvalue)))))