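; BP_Door is a procedural generation door actor that the player opens and closes with the keyboard.
; On BeginPlay it caches the Door component's position as closed, derives an open position 200 units above it, and enables player input.
; An AnyKey event compares key display names, sending W to open and S to close.
; MoveToPos snaps the whole actor to that position, without interpolation or sweep.
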(event EventBeginPlay
  (Variables|Default|SetDoorClosePos (Transformation|GetWorldLocation (Variables|Default|GetDoor)))
  (Variables|Default|SetDoorOpenPos (Math|Vector|MakeVector (.X (Math|Vector|BreakVector (Variables|Default|GetDoorClosePos))) (.Y (Math|Vector|BreakVector (Variables|Default|GetDoorClosePos))) (+ (.Z (Math|Vector|BreakVector (Variables|Default|GetDoorClosePos))) 2e+02)))
  (Input|EnableInput (Game|GetPlayerController 0)))

(event Collision|EventActorBeginOverlap
  (params (OtherActor :type Actor%20Object%20Reference)))

(event EventTick
  (params (DeltaSeconds :type Float%20%28single-precision%29)))

(event Input|KeyboardEvents|AnyKey
  (params (Key :type Key%20Structure :default "None"))
  (bind _returnvalue (Class|KismetInputLibrary|KeyGetDisplayName Key true))
  (:Pressed
    (if (Utilities|Enum|Equal(Enum) (Utilities|String|ToString(Text) _returnvalue) "W")
      (CallFunction|MovetoPos (Variables|Default|GetDoorOpenPos))
      (elif (Utilities|Enum|Equal(Enum) (Utilities|String|ToString(Text) _returnvalue) "S")
        (CallFunction|MovetoPos (Variables|Default|GetDoorClosePos))))))

(fn ConstructionScript)

(fn MovetoPos
  (params (Pos :type Vector))
  (Transformation|SetActorLocation Pos false false))