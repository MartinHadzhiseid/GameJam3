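; Inventory component that holds an actor's items in a fixed-size slot array and broadcasts updates.
; PickUp fills a matching non-full stack, else an empty slot, using stack limits, classes and sounds from DT_ItemData.
; TransferSlots merges matching stacks across inventories with overflow left at the source, but writes both sides of a swap into its own array.
; DropFromInventory clears the slot and spawns item actors in a random cone ahead of the owner.
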(event Custom|UpdateInventory
  (Default|CallOnInventoryUpdated))

(event EventBeginPlay
  (Utilities|Array|Resize (Variables|Default|GetItemSlots) (Variables|Default|GetInventorySize)))

(fn PrintInventory
  (for (_array_element _array_index) (Variables|Default|GetItemSlots)
    (Development|PrintString (Utilities|String|Append (Utilities|String|ToString(Integer) _array_index) " : " (Utilities|String|ToString(Name) (.ItemID (Utilities|Struct|BreakS_ItemSlot _array_element))) " = " (Utilities|String|ToString(Integer) (.ItemQuantity (Utilities|Struct|BreakS_ItemSlot _array_element)))))))

(fn GetItemData
  (params (ItemID :type Name))
  (bind _returnvalue (Utilities|GetDataTableRow "/Game/Inventory/ItemData/DT_ItemData.DT_ItemData" ItemID)
    (:then
      (return _returnvalue))))

(fn PickUp
  (params (ItemID :type Name) (ItemQuantity :type Integer))
  (bind (_success _index) (CallFunction|AnyAvailableSlots))
  (bind _output_get (LocalVariables|SetLocal_ItemQuantity ItemQuantity))
  (while (and (> _output_get 0) (not (LocalVariables|GetLocal_IsFull)))
    (bind (_success_2 _index_2) (CallFunction|FindMatchingSlot ItemID))
    (if _success_2
      (CallFunction|AddtoMatchingSlot _index_2 1)
      (Math|Integer|DecrementInt (LocalVariables|GetLocal_ItemQuantity) :!label _label
        (:%20%20
          (CallFunction|PlaySFX (Utilities|Struct|BreakS_ItemSFX (CallFunction|GetItemSFX ItemID)))
          (CallFunction|UpdateInventory)
          (return true 0)))
      (elif _success
        (CallFunction|AddtoNewSlot ItemID 1 _index)
        (goto _label))))
  (CallFunction|UpdateInventory)
  (return (not (LocalVariables|GetLocal_IsFull)) (LocalVariables|GetLocal_ItemQuantity)))

(fn FindMatchingSlot
  (params (ItemID :type Name))
  (for (_array_element _array_index) (Variables|Default|GetItemSlots)
    (if (and (== ItemID (.ItemID (Utilities|Struct|BreakS_ItemSlot _array_element))) (< (.ItemQuantity (Utilities|Struct|BreakS_ItemSlot _array_element)) (.SlotQuantity (Utilities|Struct|BreakS_ItemInfo (CallFunction|GetItemData ItemID)))))
      (return true _array_index)))
  (return false -1))

(fn AddtoNewSlot
  (params (ItemID :type Name) (ItemQuantity :type Integer) (Index :type Integer))
  (Utilities|Array|SetArrayElem (Variables|Default|GetItemSlots) Index (Utilities|Struct|MakeS_ItemSlot ItemID ItemQuantity)))

(fn AnyAvailableSlots
  (for (_array_element _array_index) (Variables|Default|GetItemSlots)
    (if (== (Utilities|Struct|BreakS_ItemSlot _array_element) 0)
      (return true _array_index)))
  (return false -1))

(fn AddtoMatchingSlot
  (params (Index :type Integer) (ItemQuantity :type Integer))
  (bind _itemslots (Variables|Default|GetItemSlots))
  (bind _output (Utilities|Array|Get(acopy) _itemslots Index))
  (Utilities|Array|SetArrayElem (Variables|Default|GetItemSlots) Index (Utilities|Struct|MakeS_ItemSlot (.itemid _output) (+ (.itemquantity _output) ItemQuantity))))

(fn GetItemSFX
  (params (ItemID :type Name))
  (return (Utilities|Struct|BreakS_ItemInfo (CallFunction|GetItemData ItemID))))

(fn PlaySFX
  (params (Sound :type Sound%20Base%20Object%20Reference))
  (Audio|PlaySoundatLocation Sound (Transformation|GetActorLocation (Components|GetOwner)) "0, 0, 0" 1.0 1.0 0.0 0 0 0 0))

(fn GetDropLocation
  (bind _returnvalue (Components|GetOwner))
  (return (+ (Transformation|GetActorLocation _returnvalue) (* (Math|Random|RandomUnitVectorinConeinDegrees (Transformation|GetActorForwardVector _returnvalue) 55.0) 1e+02))))

(fn DropfromInventory
  (params (ItemID :type Name) (ItemQuantity :type Integer) (Index :type Integer))
  (for _index (range 0 (- ItemQuantity 1))
    (Game|SpawnActorfromClass (Utilities|Struct|BreakS_ItemInfo (CallFunction|GetItemData ItemID)) (Math|Transform|MakeTransform (CallFunction|GetDropLocation) "0, 0, 0" "1.000000,1.000000,1.000000") "Undefined" "MultiplyWithRoot" 0 0)
    (Utilities|Array|SetArrayElem (Variables|Default|GetItemSlots) Index (Utilities|Struct|MakeS_ItemSlot "None" 0))
    (CallFunction|UpdateInventory)
    (CallFunction|PlaySFX (Utilities|Struct|BreakS_ItemSFX (CallFunction|GetItemSFX ItemID)))))

(fn TransferSlots
  (params (Index :type Integer) (SourceIndex :type Integer) (SourceInventory :type BPC%20Inventory%20Object%20Reference))
  (LocalVariables|SetLocal_DestinationInventory (Utilities|Array|Get(acopy) (Variables|Default|GetItemSlots) Index))
  (LocalVariables|SetLocal_SourceInventory (Utilities|Array|Get(acopy) (Variables|BPC_Inventory_C|GetItemSlots SourceInventory) SourceIndex))
  (Utilities|FlowControl|Sequence
    (:then_0
      (if (== (Utilities|Struct|BreakS_ItemSlot (LocalVariables|GetLocal_DestinationInventory)) (Utilities|Struct|BreakS_ItemSlot (LocalVariables|GetLocal_SourceInventory)))
        (CallFunction|ItemTransfer SourceInventory (LocalVariables|GetLocal_SourceInventory) (LocalVariables|GetLocal_DestinationInventory) Index SourceIndex)
        (else
          (CallFunction|AddtoNewSlot (.ItemID (Utilities|Struct|BreakS_ItemSlot (LocalVariables|GetLocal_DestinationInventory))) (.ItemQuantity (Utilities|Struct|BreakS_ItemSlot (LocalVariables|GetLocal_DestinationInventory))) SourceIndex)
          (CallFunction|AddtoNewSlot (.ItemID (Utilities|Struct|BreakS_ItemSlot (LocalVariables|GetLocal_SourceInventory))) (.ItemQuantity (Utilities|Struct|BreakS_ItemSlot (LocalVariables|GetLocal_SourceInventory))) Index))))
    (:then_1
      (CallFunction|UpdateInventory SourceInventory)
      (CallFunction|UpdateInventory)
      (CallFunction|PlaySFX (Utilities|Struct|BreakS_ItemSFX (CallFunction|GetItemSFX (Utilities|Struct|BreakS_ItemSlot (LocalVariables|GetLocal_SourceInventory))))))))

(fn ItemTransfer
  (params (SourceInventory :type BPC%20Inventory%20Object%20Reference) (SourceSlot :type S%20Item%20Slot%20Structure) (DestinationSlot :type S%20Item%20Slot%20Structure) (Index :type Integer) (SourceIndex :type Integer))
  (bind (_itemid _itemquantity) (Utilities|Struct|BreakS_ItemSlot SourceSlot))
  (bind _itemid_2 (Utilities|Struct|BreakS_ItemSlot SourceSlot))
  (bind _itemdata (CallFunction|GetItemData _itemid_2))
  (bind _slotquantity (Utilities|Struct|BreakS_ItemInfo _itemdata))
  (bind _output_get (LocalVariables|SetLocal_TotalSum (+ _itemquantity (Utilities|Struct|BreakS_ItemSlot DestinationSlot))))
  (if (> _output_get (Utilities|Struct|BreakS_ItemInfo (CallFunction|GetItemData _itemid)))
    (LocalVariables|SetLocal_SubtratedSum (- (LocalVariables|GetLocal_TotalSum) _slotquantity))
    (CallFunction|AddtoNewSlot (Utilities|Struct|BreakS_ItemSlot SourceSlot) _slotquantity Index)
    (CallFunction|AddtoNewSlot SourceInventory (Utilities|Struct|BreakS_ItemSlot SourceSlot) (LocalVariables|GetLocal_SubtratedSum) SourceIndex)
    (else
      (CallFunction|AddtoNewSlot (Utilities|Struct|BreakS_ItemSlot SourceSlot) (LocalVariables|GetLocal_TotalSum) Index)
      (CallFunction|AddtoNewSlot SourceInventory "None" 0 SourceIndex))))