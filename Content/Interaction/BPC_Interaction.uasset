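; Interaction component that lets its owning actor detect interactable objects ahead and interact with them.
; A looping timer runs a short forward sphere trace, storing a hit BPI_Interaction implementer as TargetActor.
; The target's LookAtMessage is shown in the player HUD's interaction widget, which is cleared when nothing qualifies.
; IA_Interact calls InteractWith on the target's BPC_ItemData component, so targets without that component only display their message.
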(event Custom|UpdateInteraction
  (CallFunction|InteractionTrace))

(event Input|EnhancedActionEvents|EnhancedInputActionIA_Interact
  (params (ActionValue :type Boolean) (ElapsedSeconds :type Float%20%28double-precision%29) (TriggeredSeconds :type Float%20%28double-precision%29) (InputAction :type Input%20Action%20Object%20Reference :default "/Game/Player/Input/Action/IA_Interact.IA_Interact"))
  (:Started
    (bind _targetactor (Variables|Default|GetTargetActor)
      (:then
        (Utilities|IsValid (Actor|GetComponentbyClass _targetactor "/Game/Inventory/ItemData/BPC_ItemData.BPC_ItemData_C")
          (:Is%20Valid
            (Default|Interactwith (Actor|GetComponentbyClass _targetactor "/Game/Inventory/ItemData/BPC_ItemData.BPC_ItemData_C") (Components|GetOwner)))))
      (:else))))

(event EventBeginPlay
  (Utilities|Time|SetTimerbyEvent (delegate Custom|UpdateInteraction) 0.1 true))

(fn GetInteractionUI
  (bind _asbp_controller (Utilities|Casting|CastToBP_Controller (Game|GetPlayerController 0)))
  (return (Variables|/Game/Interaction/UI/WB_PlayerHUD.WB_PlayerHUD_C|GetWB_InteractionUI (Variables|/Game/Player/BP_Controller.BP_Controller_C|GetWB_PlayerHUD _asbp_controller))))

(fn InteractionTrace
  (bind _returnvalue (Components|GetOwner))
  (bind _returnvalue_2 (Transformation|GetActorLocation _returnvalue))
  (bind (_outhit _returnvalue_3) (Collision|SphereTraceByChannel _returnvalue_2 (+ _returnvalue_2 (* (Transformation|GetActorForwardVector _returnvalue) 1e+02)) 7e+01 "TraceTypeQuery3" false 0 "None"))
  (if _returnvalue_3
    (if (Utilities|DoesObjectImplementInterface (.HitActor (Collision|BreakHitResult _outhit)) "/Game/Interaction/BPI_Interaction.BPI_Interaction_C")
      (bind _output_get (Variables|Default|SetTargetActor (.HitActor (Collision|BreakHitResult _outhit))))
      (bind _message (Class|BPIInteraction|Lookat(Message) _output_get))
      (Default|SetMessage (CallFunction|GetInteractionUI) _message)
      (else
        (Variables|Default|SetTargetActor 0)
        (Default|SetMessage (CallFunction|GetInteractionUI))))
    (else
      (Variables|Default|SetTargetActor 0)
      (Default|SetMessage (CallFunction|GetInteractionUI)))))