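; Player character Blueprint for Duff McKagan, with movement locked to world X, jumping, climbing, combat and death.
; Enhanced Input drives the actions, and any actor overlap switches to gravity-free flying for vertical climbing until overlap ends.
; Attack and special montages briefly enable hitboxes that apply damage on overlap, with a cooldown on the special.
; Parrying blocks incoming damage, though its overlap response is empty; zero health disables input and destroys the actor after a montage.
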(event OnComponentBeginOverlap(Hitbox)
  (params (OverlappedComponent :type Primitive%20Component%20Object%20Reference) (OtherActor :type Actor%20Object%20Reference) (OtherComp :type Primitive%20Component%20Object%20Reference) (OtherBodyIndex :type Integer) (bFromSweep :type Boolean) (SweepResult :type Hit%20Result%20Structure%20%28by%20ref%29))
  ;[0.15 0.15 0.15 0.5] Main Attack
  (Game|Damage|ApplyDamage OtherActor (Variables|Default|GetMainAttackDamage) 0 0))

(event OnComponentBeginOverlap(SpecialAttackHitbox)
  (params (OverlappedComponent :type Primitive%20Component%20Object%20Reference) (OtherActor :type Actor%20Object%20Reference) (OtherComp :type Primitive%20Component%20Object%20Reference) (OtherBodyIndex :type Integer) (bFromSweep :type Boolean) (SweepResult :type Hit%20Result%20Structure%20%28by%20ref%29))
  ;[0.15 0.15 0.15 0.5] Special Attack
  (Game|Damage|ApplyDamage OtherActor (Variables|Default|GetSpecialAttackDamage) 0 0))

(event OnComponentBeginOverlap(ParryBox)
  (params (OverlappedComponent :type Primitive%20Component%20Object%20Reference) (OtherActor :type Actor%20Object%20Reference) (OtherComp :type Primitive%20Component%20Object%20Reference) (OtherBodyIndex :type Integer) (bFromSweep :type Boolean) (SweepResult :type Hit%20Result%20Structure%20%28by%20ref%29)))

(event Input|EnhancedActionEvents|EnhancedInputActionIA_Attack
  (params (ActionValue :type Boolean) (ElapsedSeconds :type Float%20%28double-precision%29) (TriggeredSeconds :type Float%20%28double-precision%29) (InputAction :type Input%20Action%20Object%20Reference :default "/Game/Player/Input/Action/IA_Attack.IA_Attack"))
  ;[0.15 0.15 0.15 0.5] Main Attack
  (if (== (Variables|Default|GetIsMainAttacking) false)
    (Variables|Default|SetIsMainAttacking true)
    (Animation|PlayAnimMontage 0 1.0 "None")
    (Collision|SetCollisionEnabled (Variables|Default|GetHitbox) "QueryOnly")
    (Utilities|FlowControl|Delay 0.2)
    (Collision|SetCollisionEnabled (Variables|Default|GetHitbox) "NoCollision")
    (Variables|Default|SetIsMainAttacking false)))

(event Input|EnhancedActionEvents|EnhancedInputActionIA_Climb
  (params (ActionValue :type Float%20%28double-precision%29) (ElapsedSeconds :type Float%20%28double-precision%29) (TriggeredSeconds :type Float%20%28double-precision%29) (InputAction :type Input%20Action%20Object%20Reference :default "/Game/Player/Input/Action/IA_Climb.IA_Climb"))
  ;[0.15 0.15 0.15 0.5] Climbing Up/Down
  (if (Variables|Default|GetIsClimbing)
    (Pawn|Input|AddMovementInput "0.000000,0.000000,1.000000" (* ActionValue (Variables|Default|GetClimbingSpeed)) false)))

(event Input|EnhancedActionEvents|EnhancedInputActionIA_Move
  (params (ActionValue :type Float%20%28double-precision%29) (ElapsedSeconds :type Float%20%28double-precision%29) (TriggeredSeconds :type Float%20%28double-precision%29) (InputAction :type Input%20Action%20Object%20Reference :default "/Game/Player/Input/Action/IA_Move.IA_Move"))
  (bind _mesh (Variables|Character|GetMesh))
  ;[0.15 0.15 0.15 0.5] Movment Left/Right and Rotating
  (Pawn|Input|AddMovementInput "1.000000,0.000000,0.000000" ActionValue false)
  (if (> ActionValue 0.0)
    (Transformation|SetRelativeRotation _mesh "0.000000,90.000000,0.000000" false false)
    (else
      (Transformation|SetRelativeRotation _mesh "0.000000,-90.000000,0.000000" false false))))

(event Input|EnhancedActionEvents|EnhancedInputActionIA_Jump
  (params (ActionValue :type Boolean) (ElapsedSeconds :type Float%20%28double-precision%29) (TriggeredSeconds :type Float%20%28double-precision%29) (InputAction :type Input%20Action%20Object%20Reference :default "/Game/Player/Input/Action/IA_Jump.IA_Jump"))
  ;[0.15 0.15 0.15 0.5] Jumping
  (:Triggered
    (Character|Jump))
  (:Completed
    (Character|StopJumping)))

(event Input|EnhancedActionEvents|EnhancedInputActionIA_Special
  (params (ActionValue :type Boolean) (ElapsedSeconds :type Float%20%28double-precision%29) (TriggeredSeconds :type Float%20%28double-precision%29) (InputAction :type Input%20Action%20Object%20Reference :default "/Game/Player/Input/Action/IA_Special.IA_Special"))
  ;[0.15 0.15 0.15 0.5] Special Attack
  (if (== (Variables|Default|GetIsSpecialAttacking) false)
    (Variables|Default|SetIsSpecialAttacking true)
    (Animation|PlayAnimMontage 0 1.0 "None")
    (Collision|SetCollisionEnabled (Variables|Default|GetSpecialAttackHitbox) "QueryOnly")
    (Utilities|FlowControl|Delay 0.2)
    (Collision|SetCollisionEnabled (Variables|Default|GetSpecialAttackHitbox) "NoCollision")
    (Utilities|FlowControl|Delay (Variables|Default|GetSpecialAttackCooldown))
    (Variables|Default|SetIsSpecialAttacking false)))

(event Input|EnhancedActionEvents|EnhancedInputActionIA_Parry
  (params (ActionValue :type Boolean) (ElapsedSeconds :type Float%20%28double-precision%29) (TriggeredSeconds :type Float%20%28double-precision%29) (InputAction :type Input%20Action%20Object%20Reference :default "/Game/Player/Input/Action/IA_Parry.IA_Parry"))
  ;[0.15 0.15 0.15 0.5] Parry
  (if (== (Variables|Default|GetIsParrying) false)
    (Variables|Default|SetIsParrying true)
    (Animation|PlayAnimMontage 0 1.0 "None")
    (Collision|SetCollisionEnabled (Variables|Default|GetParryBox) "QueryOnly")
    (Utilities|FlowControl|Delay 0.3)
    (Collision|SetCollisionEnabled (Variables|Default|GetParryBox) "NoCollision")
    (Variables|Default|SetIsParrying false)))

(event EventBeginPlay
  (Input|AddMappingContext (PlayerController|LocalPlayerSubsystems|GetEnhancedInputLocalPlayerSubsystem (Game|GetPlayerController 0)) "/Game/Player/Input/IMC_Default.IMC_Default" 0 "(bIgnoreAllPressedKeysUntilRelease=True,bForceImmediately=False,bNotifyUserSettings=False)"))

(event Collision|EventActorBeginOverlap
  (params (OtherActor :type Actor%20Object%20Reference))
  (bind _charactermovement (Variables|Character|GetCharacterMovement))
  ;[0.15 0.15 0.15 0.5] Temporarily disable gravity while character is climbing
  (Variables|Default|SetIsClimbing true)
  (Variables|/Script/Engine.CharacterMovementComponent|SetGravityScale _charactermovement 0.0)
  (Pawn|Components|CharacterMovement|SetMovementMode _charactermovement "MOVE_Flying" 0))

(event Collision|EventActorEndOverlap
  (params (OtherActor :type Actor%20Object%20Reference))
  (bind _charactermovement (Variables|Character|GetCharacterMovement))
  ;[0.15 0.15 0.15 0.5] Temporarily disable gravity while character is climbing
  (Variables|Default|SetIsClimbing false)
  (Variables|/Script/Engine.CharacterMovementComponent|SetGravityScale _charactermovement 1.0)
  (Pawn|Components|CharacterMovement|SetMovementMode _charactermovement "MOVE_Walking" 0))

(event EventApplyDamage
  (params (DamageAmount :type Float%20%28double-precision%29))
  ;[0.15 0.15 0.15 0.5] Taking Damage and handling death
  (if (not (Variables|Default|GetIsParrying))
    (bind _output_get (Variables|Default|SetCurrentHealth (Math|Float|Clamp(Float) (- (Variables|Default|GetCurrentHealth) DamageAmount) 0.0 (Variables|Default|GetMaxHealth))))
    (if (<= _output_get 0.0)
      (Input|DisableInput (Game|GetPlayerController 0))
      (Animation|PlayAnimMontage 0 1.0 "None")
      (Utilities|FlowControl|Delay 2.0)
      (Actor|DestroyActor))))

(fn ConstructionScript)