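; Player controller Blueprint that owns the player's HUD and inventory screen.
; On BeginPlay it creates the player HUD widget and adds it to the viewport.
; The inventory input toggles the inventory UI, removing and clearing the existing widget or creating a new one.
; A new inventory widget is only created if the player character has a BPC_Inventory component, which is passed into it.
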(event Input|EnhancedActionEvents|EnhancedInputActionIA_Inventory
  (params (ActionValue :type Boolean) (ElapsedSeconds :type Float%20%28double-precision%29) (TriggeredSeconds :type Float%20%28double-precision%29) (InputAction :type Input%20Action%20Object%20Reference :default "/Game/Player/Input/Action/IA_Inventory.IA_Inventory"))
  (:Started
    (bind _wb_inventoryui (Variables|Default|GetWB_InventoryUI)
      (:then
        (Widget|RemovefromParent _wb_inventoryui)
        (Variables|Default|SetWB_InventoryUI 0)
        (Development|PrintString "Inventory Closed"))
      (:else
        (CallFunction|DisplayInventoryUI)
        (Development|PrintString "Inventory Opened")))))

(event EventBeginPlay
  (CallFunction|DisplayPlayerHUD))

(fn ConstructionScript)

(fn DisplayPlayerHUD
  (bind _returnvalue (UserInterface|CreateWidget "/Game/Interaction/UI/WB_PlayerHUD.WB_PlayerHUD_C"))
  (bind _output_get (Variables|Default|SetWB_PlayerHUD _returnvalue))
  (UserInterface|Viewport|AddtoViewport _output_get 0))

(fn DisplayInventoryUI
  (bind _returnvalue (Game|GetPlayerCharacter 0))
  (bind _returnvalue_2 (Actor|GetComponentbyClass _returnvalue "/Game/Inventory/BPC_Inventory.BPC_Inventory_C"))
  (Utilities|IsValid _returnvalue_2
    (:Is%20Valid
      (bind _returnvalue_3 (UserInterface|CreateWidget "/Game/Inventory/UI/WB_InventoryUI.WB_InventoryUI_C" 0 _returnvalue_2))
      (bind _output_get (Variables|Default|SetWB_InventoryUI _returnvalue_3))
      (UserInterface|Viewport|AddtoViewport _output_get 0))))